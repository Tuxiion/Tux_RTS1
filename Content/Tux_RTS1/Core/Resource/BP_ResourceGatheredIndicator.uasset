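; BP_ResourceGatheredIndicator is a short-lived actor that shows a mesh rising upward, apparently as feedback when a resource is gathered.
; The construction script sets the mesh from the MeshToUse variable.
; On BeginPlay, a sped-up timeline scales MaxUpwardsdistance to move the mesh along relative Z, then destroys the actor when it finishes.
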(event EventBeginPlay
  (Components|Timeline|SetPlayRate (Variables|Default|GetUpwards%20Animation) 1.7)
  (bind _zvaluealpha (Timeline|Upwards%20Animation Play)
    (:Update
      (Transformation|SetRelativeLocation (Variables|Default|GetResourceMesh) (Math|Vector|MakeVector 0.0 0.0 (* _zvaluealpha (Variables|Default|GetMaxUpwardsdistance))) false false))
    (:Finished
      (Actor|DestroyActor))))

(event Collision|EventActorBeginOverlap
  (params (OtherActor :type Actor%20Object%20Reference)))

(event EventTick
  (params (DeltaSeconds :type Float%20%28single-precision%29)))

(fn ConstructionScript
  (Components|StaticMesh|SetStaticMesh (Variables|Default|GetResourceMesh) (Variables|Default|GetMeshToUse)))