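; RTS player controller that handles camera movement, unit selection, orders and the player's resource stockpile.
; Movement axes pan the controlled pawn, falling back to screen-edge mouse scrolling when idle.
; Mouse actions drive a spawned selection marquee and, on release, send selected actors move, gather or building-interact orders through interfaces, chosen by a sphere overlap at the cursor.
; ReceiveResources accumulates amounts per type and updates the HUD.
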(event Custom|AddActorSelectedToList
  (params (SelectedActor :type Actor%20Object%20Reference))
  (CallFunction|DeselectAllActors)
  (Utilities|Array|Add (Variables|Default|GetSelectedActors) SelectedActor))

(event Custom|DeselectAllActors
  (for _array_element (Variables|Default|GetSelectedActors)
    (if (Utilities|DoesObjectImplementInterface _array_element "/Game/Tux_RTS1/Core/Building/BPI_SelectionEvents.BPI_SelectionEvents_C")
      (Class|BPISelectionEvents|DeselectThis(Message) _array_element)))
  (Utilities|Array|Clear (Variables|Default|GetSelectedActors)))

(event EventBeginPlay
  (bind _returnvalue (Game|SpawnActorfromClass "/Game/Tux_RTS1/Core/Player/BP_UnitSelectionMarquee.BP_UnitSelectionMarquee_C" (Math|Transform|MakeTransform "0, 0, 0" "0, 0, 0" "1.000000,1.000000,1.000000") "Undefined" 0 0))
  (Variables|Default|SetSelectionMarqueeRef _returnvalue))

(event EventTick
  (params (DeltaSeconds :type Float%20%28single-precision%29)))

(event Input|ActionEvents|InputActionMouseAction
  (params (Key :type Key%20Structure :default "None"))
  (bind _hitresult (Game|Player|GetHitResultUnderCursorbyChannel "TraceTypeQuery1" true))
  (bind _location (Collision|BreakHitResult _hitresult))
  (:Released
    (if (Utilities|Array|IsNotEmpty (Variables|Default|GetSelectedActors))
      (bind _outactors (Collision|SphereOverlapActors (.Location (Collision|BreakHitResult (.HitResult (Game|Player|GetHitResultUnderCursorbyChannel "TraceTypeQuery1" true)))) 1e+02 (Utilities|Array|MakeArray "ObjectTypeQuery2" "ObjectTypeQuery3") 0))
      (if (Utilities|Array|IsEmpty _outactors)
        ;[1 1 1] Unit movement
        (for _array_element (Variables|Default|GetSelectedActors)
          (if (Utilities|DoesObjectImplementInterface _array_element "/Game/Tux_RTS1/Core/Unit/BPI_UnitActions.BPI_UnitActions_C")
            (Class|BPIUnitActions|MovetoThisLocation(Message) _array_element _location)
            (Niagara|SpawnSystematLocation "/Game/Tux_RTS1/Core/Player/NS_ClickIndicator.NS_ClickIndicator" _location)))
        (else
          (for _array_element_2 (Variables|Default|GetSelectedActors)
            (if (Utilities|DoesObjectImplementInterface _array_element_2 "/Game/Tux_RTS1/Core/Unit/BPI_UnitActions.BPI_UnitActions_C")
              (if (Utilities|IsValid (Actor|GetComponentbyClass (Utilities|Array|Get(acopy) _outactors) "/Game/Tux_RTS1/Core/Resource/BP_ResourceComponent.BP_ResourceComponent_C"))
                (Class|BPIUnitActions|GatherThisResource(Message) _array_element_2 (Utilities|Array|Get(acopy) _outactors))
                (elif (Utilities|IsValid (Actor|GetComponentbyClass (Utilities|Array|Get(acopy) _outactors) "/Game/Tux_RTS1/Core/Building/BP_BuildingComponent.BP_BuildingComponent_C"))
                  (Class|BPIUnitActions|InteractwithBuilding(Message) _array_element_2 (Utilities|Array|Get(acopy) _outactors)))))))))))

(event Input|ActionEvents|InputActionMouseAction
  (params (Key :type Key%20Structure :default "None"))
  (:Pressed
    (Transformation|SetActorLocation (Variables|Default|GetSelectionMarqueeRef) (.Location (Collision|BreakHitResult (.HitResult (Game|Player|GetHitResultUnderCursorbyChannel "TraceTypeQuery1" true)))) false false)
    (Default|StartResizingMarquee (Variables|Default|GetSelectionMarqueeRef)))
  (:Released
    (Default|EndResizingMarquee (Variables|Default|GetSelectionMarqueeRef))))

(event Input|AxisEvents|InputAxisMoveForward
  (params (AxisValue :type Float%20%28single-precision%29))
  ;[1 1 1] Camera movement
  (Pawn|Input|AddMovementInput (Pawn|GetControlledPawn) (Math|Vector|GetForwardVector (Math|Rotator|MakeRotator 0.0 0.0 (.yaw (Pawn|GetControlRotation :!class /Script/Engine.Controller)))) (Math|Float|SelectFloat AxisValue (Variables|Default|GetMouseForwardScale) (!= AxisValue 0.0)) false))

(event Input|AxisEvents|InputAxisMoveRight
  (params (AxisValue :type Float%20%28single-precision%29))
  ;[1 1 1] Camera movement
  (Pawn|Input|AddMovementInput (Pawn|GetControlledPawn) (Math|Vector|GetRightVector (Math|Rotator|MakeRotator 0.0 0.0 (.yaw (Pawn|GetControlRotation :!class /Script/Engine.Controller)))) (Math|Float|SelectFloat AxisValue (Variables|Default|GetMouseRightScale) (!= AxisValue 0.0)) false))

(event Input|AxisEvents|InputAxisMouseMovement
  (params (AxisValue :type Float%20%28single-precision%29))
  (bind _locationy (Game|Player|GetMousePosition))
  (bind _returnvalue (Viewport|GetViewportSize))
  (bind _locationx (Game|Player|GetMousePosition))
  (bind _returnvalue_2 (Viewport|GetViewportSize))
  (bind _returnvalue_3 (/ _locationx (.x _returnvalue_2)))
  (bind _returnvalue_4 (/ _locationy (.y _returnvalue)))
  ;[1 1 1] Camera movement
  (Variables|Default|SetMouseRightScale (Math|Float|SelectFloat -1.0 (Math|Float|SelectFloat 1.0 0.0 (> _returnvalue_3 (- 1.0 (Variables|Default|GetViewport%20Edge%20Threshold)))) (< _returnvalue_3 (Variables|Default|GetViewport%20Edge%20Threshold))))
  (Variables|Default|SetMouseForwardScale (Math|Float|SelectFloat 1.0 (Math|Float|SelectFloat -1.0 0.0 (> _returnvalue_4 (- 1.0 (Variables|Default|GetViewport%20Edge%20Threshold)))) (< _returnvalue_4 (Variables|Default|GetViewport%20Edge%20Threshold)))))

(fn ConstructionScript)

(fn ReceiveResources
  (params (Type :type E_ResourceType%20Enum :default "NewEnumerator0") (Amount :type Integer))
  (Utilities|FlowControl|Sequence
    (:then_0
      (if (Utilities|Map|Contains (Variables|Default|GetStoredResources) Type)
        (Utilities|Map|Add (Variables|Default|GetStoredResources) Type (+ (.Value (Utilities|Map|Find (Variables|Default|GetStoredResources) Type)) Amount))
        (else
          (Utilities|Map|Add (Variables|Default|GetStoredResources) Type Amount))))
    (:then_1
      (bind _asbp_hud (Utilities|Casting|CastToBP_HUD (HUD|GetHUD)))
      (Default|UpdateResourceValue (Variables|/Game/Tux_RTS1/Core/Player/BP_HUD.BP_HUD_C|GetHUDWidgetRef _asbp_hud) Type (.Value (Utilities|Map|Find (Variables|Default|GetStoredResources) Type))))))