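; BP_UnitSelectionMarquee is an RTS actor for a unit selection marquee, though so far it only moves its Sphere component to follow the cursor.
; StartResizingMarquee and EndResizingMarquee toggle a flag that gates Tick.
; While the flag is set, Tick gets the PC_Tux_RTS1 player controller and places the Sphere at its complex Visibility trace hit under the cursor.
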(event EventBeginPlay)

(event Collision|EventActorBeginOverlap
  (params (OtherActor :type Actor%20Object%20Reference)))

(event EventTick
  (params (DeltaSeconds :type Float%20%28single-precision%29))
  (if (Variables|Default|GetShouldResizeMarquee)
    (bind _aspc_tux_rts1 (Utilities|Casting|CastToPC_Tux_RTS1 (Game|GetPlayerController 0)))
    (Transformation|SetWorldLocation (Variables|Default|GetSphere) (.Location (Collision|BreakHitResult (.HitResult (Game|Player|GetHitResultUnderCursorbyChannel _aspc_tux_rts1 "TraceTypeQuery1" true)))) false false)))

(fn ConstructionScript)

(fn StartResizingMarquee
  (Variables|Default|SetShouldResizeMarquee true))

(fn EndResizingMarquee
  (Variables|Default|SetShouldResizeMarquee false))